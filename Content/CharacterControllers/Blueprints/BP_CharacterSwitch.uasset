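; BP_CharacterSwitch is a controller Blueprint that lets the player cycle possession between the third-person characters in the level.
; BeginPlay caches all BP_ThirdPersonCharacter actors as a roster and records the player's starting character as current.
; Pressing E calls NextCharacter, which finds the current character's index, advances it, wraps to zero past the end, and possesses that character.
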(event `self.ReceiveBeginPlay`
  (bind _outactors (`GameplayStatics.GetAllActorsOfClass` "/Game/CharacterControllers/Blueprints/BP_ThirdPersonCharacter.BP_ThirdPersonCharacter_C"))
  (set `self.CharacterRoster` _outactors)
  (bind _asbp_third_person_character (cast `/Game/CharacterControllers/Blueprints/BP_ThirdPersonCharacter` (`GameplayStatics.GetPlayerCharacter` 0)))
  (set `self.CurrentCharacter` _asbp_third_person_character))

(event `Key|E`
  (params (Key :type "Key Structure"))
  (:`Pressed`
    (`self.NextCharacter`)))

(fn `NextCharacter`
  (locals (Local_Index :type Integer))
  (bind _returnvalue (`KismetArrayLibrary.Array_Find` (`self.CharacterRoster`) (`self.CurrentCharacter`)))
  (bind _returnvalue_2 (+ _returnvalue 1))
  (set `local.Local_Index` _returnvalue)
  (bind _output_get (set `local.Local_Index` (`KismetMathLibrary.SelectInt` _returnvalue_2 0 (`KismetArrayLibrary.Array_IsValidIndex` (`self.CharacterRoster`) _returnvalue_2))))
  (bind _output_get_2 (set `self.CurrentCharacter` (`|GetArrayItem` (`self.CharacterRoster`) _output_get)))
  (`self.Possess` _output_get_2))

(fn `UserConstructionScript`)